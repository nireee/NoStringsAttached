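; Camera actor with a cine camera and spring arm that follows the third-person player and can focus on a target.
; While Followed is set, Tick places it at the player mesh location plus a configurable offset.
; FocusObj turns following off, lerps the actor toward the target plus that offset, then calls ZoomIn.
; ZoomIn blends spring arm length and rotates toward the target using a caller-supplied alpha.
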(event Custom|Set%20Cam%20Distance
  (params (distance :type Vector))
  (Variables|Default|Setcam_distance_from_player distance))

(event EventBeginPlay
  (bind _asbp_third_person_character (Utilities|Casting|CastToBP_ThirdPersonCharacter (Game|GetPlayerCharacter 0)))
  (Variables|Default|SetPlayer _asbp_third_person_character)
  (Input|EnableInput (Game|GetPlayerController 0)))

(event Collision|EventActorBeginOverlap
  (params (OtherActor :type Actor%20Object%20Reference)))

(event EventTick
  (params (DeltaSeconds :type Float%20%28single-precision%29))
  (bind _player (Variables|Default|GetPlayer))
  (bind _cam_distance_from_player (Variables|Default|Getcam_distance_from_player))
  (bind _mesh (Variables|/Script/Engine.Character|GetMesh _player))
  (bind _returnvalue (Transformation|GetWorldLocation _mesh))
  (bind _returnvalue_2 (+ _returnvalue _cam_distance_from_player))
  (if (Variables|Default|GetFollowed?)
    (Transformation|SetActorLocation (Components|GetOwner (Variables|Default|GetCineCamera)) (Math|Vector|MakeVector (.x _returnvalue_2) (.y _returnvalue_2) (.z _returnvalue_2)) false false)))

(fn ConstructionScript)

(fn Zoomin
  (params (Target%20Distance :type Float%20%28double-precision%29) (Default%20Distance :type Float%20%28double-precision%29) (Alpha :type Float%20%28double-precision%29) (Target%20To%20Focus :type Vector) (Init%20Rot :type Rotator))
  ;[1 1 1] Zoom In and focus on target
  (Variables|/Script/Engine.SpringArmComponent|SetTargetArmLength (Variables|Default|GetSpringArm) (Math|Float|Lerp Default%20Distance Target%20Distance Alpha))
  (Transformation|SetActorRotation (Math|Rotator|Lerp(Rotator) Init%20Rot (Math|Rotator|FindLookatRotation (Transformation|GetActorLocation) Target%20To%20Focus) Alpha)))

(fn FocusObj
  (params (TargetLoc :type Vector) (Expect_SpringArm_Length :type Float%20%28double-precision%29) (Alpha :type Float%20%28double-precision%29))
  (bind _cinecamera (Variables|Default|GetCineCamera))
  (bind _cam_distance_from_player (Variables|Default|Getcam_distance_from_player))
  (bind _returnvalue (Components|GetOwner _cinecamera))
  (bind _returnvalue_2 (+ TargetLoc _cam_distance_from_player))
  (bind _returnvalue_3 (Transformation|GetActorLocation _returnvalue))
  (bind _returnvalue_4 (Math|Vector|Lerp(Vector) _returnvalue_3 (Math|Vector|MakeVector (.x _returnvalue_2) (.y _returnvalue_2) (.z _returnvalue_2)) Alpha))
  (Variables|Default|SetFollowed? false)
  (Transformation|SetActorLocation _returnvalue (Math|Vector|MakeVector (.x _returnvalue_4) (.y _returnvalue_4) (.z _returnvalue_4)) false false)
  (CallFunction|Zoomin Expect_SpringArm_Length (Variables|Default|GetInit_SpringArmLength) Alpha TargetLoc (Variables|Default|GetInit_Rotation)))