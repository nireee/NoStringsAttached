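; CamSwitchRegion is a region actor that switches the player's camera when an actor begins overlapping it.
; On BeginPlay it caches the BP_ThirdPersonCharacter found by class lookup.
; Any overlap, with no check on the overlapping actor, passes UpdatedCamNum to that character's SwitchCam, then disables its input for a one-second delay.
; Ending the overlap does nothing, and a duplicate chain using CamNum is left unconnected.
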(event EventBeginPlay
  (bind _returnvalue (Actor|GetActorOfClass "/Game/ThirdPerson/Blueprints/BP_ThirdPersonCharacter.BP_ThirdPersonCharacter_C"))
  (Variables|Default|SetPlayer _returnvalue))

(event Collision|EventActorBeginOverlap
  (params (OtherActor :type Actor%20Object%20Reference))
  (bind _returnvalue (Game|GetPlayerController 0))
  (bind _player (Variables|Default|GetPlayer))
  (Default|SwitchCam _player (Variables|Default|GetUpdatedCamNum))
  (Input|DisableInput _player _returnvalue)
  (Utilities|FlowControl|Delay 1.0)
  (Input|EnableInput _player _returnvalue))

(event EventTick
  (params (DeltaSeconds :type Float%20%28single-precision%29)))

(event Collision|EventActorEndOverlap
  (params (OtherActor :type Actor%20Object%20Reference)))

(fn ConstructionScript)