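; FixedCam is a camera actor that follows the third-person player character at a fixed offset, without changing its own rotation.
; On BeginPlay it caches the player character and enables input from the first player controller.
; Every Tick it moves the CineCamera's owning actor to the player mesh's world location plus CamDistanceFromPlayer, with no interpolation or sweep.
; The SetCamDistance event replaces that offset at runtime.
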(event Custom|Set%20Cam%20Distance
  (params (distance :type Vector))
  (Variables|Default|Setcam_distance_from_player distance))

(event EventBeginPlay
  (bind _asbp_third_person_character (Utilities|Casting|CastToBP_ThirdPersonCharacter (Game|GetPlayerCharacter 0)))
  (Variables|Default|SetPlayer _asbp_third_person_character)
  (Input|EnableInput (Game|GetPlayerController 0)))

(event Collision|EventActorBeginOverlap
  (params (OtherActor :type Actor%20Object%20Reference)))

(event EventTick
  (params (DeltaSeconds :type Float%20%28single-precision%29))
  (Transformation|SetActorLocation (Components|GetOwner (Variables|Default|GetCineCamera)) (+ (Transformation|GetWorldLocation (Variables|/Script/Engine.Character|GetMesh (Variables|Default|GetPlayer))) (Variables|Default|Getcam_distance_from_player)) false false))

(fn ConstructionScript)