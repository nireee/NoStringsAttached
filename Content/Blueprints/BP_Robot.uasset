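; BP_Robot is a robot Blueprint that picks up and drops pills using a physics constraint.
; PickUpPills sphere-traces around the actor for a PhysicsBody object and constrains the hit component to the ControlPanel.
; A failed trace clears InteractButton's Pickup flag, and LeavePills breaks the constraint to release the held object.
; Debug trace drawing and print strings are left on; BeginPlay, overlap and Tick are empty.
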(event Custom|PickUpPills
  (bind _returnvalue (Transformation|GetActorLocation))
  (bind (_outhit _returnvalue_2) (Collision|SphereTraceForObjects _returnvalue _returnvalue 1.5e+02 (Utilities|Array|MakeArray "ObjectTypeQuery4") false 0 "ForDuration"))
  (if _returnvalue_2
    (Class|PhysicsConstraintComponent|SetConstrainedComponents (Variables|Default|GetPhysicsConstraint) (Variables|Default|GetControlPanel) "None" (.hitcomponent _outhit) "None")
    (Development|PrintString (Utilities|GetDisplayName (.hitcomponent _outhit)))
    (else
      (Variables|/Game/Blueprints/ControllerButton.ControllerButton_C|Setpickup (Variables|Default|Getinteract_button) false)
      (Development|PrintString "not pickup"))))

(event Custom|LeavePills
  (Class|PhysicsConstraintComponent|BreakConstraint (Variables|Default|GetPhysicsConstraint)))

(event EventBeginPlay)

(event Collision|EventActorBeginOverlap
  (params (OtherActor :type Actor%20Object%20Reference)))

(event EventTick
  (params (DeltaSeconds :type Float%20%28single-precision%29)))

(fn ConstructionScript)