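; Circus act seesaw that lets the player and one designated object launch each other upward from opposite ends.
; Left and right surface overlaps track whether the player character and RightObject are in place.
; When one lands while the other is present, the other receives a PushUpBySeeSaw interface message, with high or low force chosen by the lander's fall speed.
; The player only triggers a launch when moving downward past a small threshold.
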(event OnComponentBeginOverlap(SurfaceLeft)
  (params (OverlappedComponent :type Primitive%20Component%20Object%20Reference) (OtherActor :type Actor%20Object%20Reference) (OtherComp :type Primitive%20Component%20Object%20Reference) (OtherBodyIndex :type Integer) (bFromSweep :type Boolean) (SweepResult :type Hit%20Result%20Structure%20%28by%20ref%29))
  (bind _rightobject (Variables|Default|GetRightObject))
  (if (== (Variables|Default|GetLeftPlayer) OtherActor)
    (Variables|Default|SetplayerIN? true)
    (if (Variables|Default|GetcubeIN?)
      (bind _leftplayer (Variables|Default|GetLeftPlayer)
        (:then
          (if (< (.z (Transformation|GetVelocity _leftplayer)) -1e+01)
            (if (< (.z (Transformation|GetVelocity _leftplayer)) (Variables|Default|GetfallSpeed))
              (Class|BPISeeSaw|PushUpbySeeSaw(Message) _rightobject (Variables|Default|GetHighPushForce_0))
              (else
                (Class|BPISeeSaw|PushUpbySeeSaw(Message) _rightobject (Variables|Default|GetLowPushForce_0))))))
        (:else)))))

(event OnComponentEndOverlap(SurfaceLeft)
  (params (OverlappedComponent :type Primitive%20Component%20Object%20Reference) (OtherActor :type Actor%20Object%20Reference) (OtherComp :type Primitive%20Component%20Object%20Reference) (OtherBodyIndex :type Integer))
  (if (== (Variables|Default|GetLeftPlayer) OtherActor)
    (Variables|Default|SetplayerIN? false)))

(event OnComponentEndOverlap(SurfaceRight)
  (params (OverlappedComponent :type Primitive%20Component%20Object%20Reference) (OtherActor :type Actor%20Object%20Reference) (OtherComp :type Primitive%20Component%20Object%20Reference) (OtherBodyIndex :type Integer))
  (if (== (Variables|Default|GetRightObject) OtherActor)
    (Variables|Default|SetcubeIN? false)))

(event OnComponentBeginOverlap(SurfaceRight)
  (params (OverlappedComponent :type Primitive%20Component%20Object%20Reference) (OtherActor :type Actor%20Object%20Reference) (OtherComp :type Primitive%20Component%20Object%20Reference) (OtherBodyIndex :type Integer) (bFromSweep :type Boolean) (SweepResult :type Hit%20Result%20Structure%20%28by%20ref%29))
  (bind _leftplayer (Variables|Default|GetLeftPlayer))
  (if (== OtherActor (Variables|Default|GetRightObject))
    (Variables|Default|SetcubeIN? true)
    (if (Variables|Default|GetplayerIN?)
      (bind _rightobject (Variables|Default|GetRightObject)
        (:then
          (if (< (.z (Transformation|GetComponentVelocity (Variables|/Game/ThirdPerson/Blueprints/EnvironmentObjects/Hidden/BP_ObjectWithWeight.BP_ObjectWithWeight_C|GetStaticMesh _rightobject))) (Variables|Default|GetfallSpeed_0))
            (Class|BPISeeSaw|PushUpbySeeSaw(Message) _leftplayer (Variables|Default|GetHighPushForce))
            (else
              (Class|BPISeeSaw|PushUpbySeeSaw(Message) _leftplayer (Variables|Default|GetLowPushForce)))))
        (:else)))))

(event EventBeginPlay
  (|CallParentFunction)
  (bind _asbp_third_person_character (Utilities|Casting|CastToBP_ThirdPersonCharacter (Game|GetPlayerCharacter 0)))
  (Variables|Default|SetLeftPlayer _asbp_third_person_character))

(event Collision|EventActorBeginOverlap
  (params (OtherActor :type Actor%20Object%20Reference))
  (|CallParentFunction OtherActor) ; This node is disabled and will not be called.\nDrag off pins to build functionality.
)

(event EventTick
  (params (DeltaSeconds :type Float%20%28single-precision%29))
  (|CallParentFunction DeltaSeconds) ; This node is disabled and will not be called.\nDrag off pins to build functionality.
)

(fn ConstructionScript
  (|CallParentFunction))