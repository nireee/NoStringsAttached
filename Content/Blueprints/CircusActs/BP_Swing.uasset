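; BP_Swing is a grabbable circus swing with a physics-driven board, optionally attached to a switch's cube at BeginPlay.
; Overlapping a "swing_box" component sends GrabSwingMessage to that actor and disables the collider, which re-enables one second after overlap ends.
; Helper functions push the board by adding clamped Y velocity or applying acceleration force.
; The cable-length, constraint-limit and looping auto-swing timer setup is disconnected, so it never runs.
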(event OnComponentBeginOverlap(Collider)
  (params (OverlappedComponent :type Primitive%20Component%20Object%20Reference) (OtherActor :type Actor%20Object%20Reference) (OtherComp :type Primitive%20Component%20Object%20Reference) (OtherBodyIndex :type Integer) (bFromSweep :type Boolean) (SweepResult :type Hit%20Result%20Structure%20%28by%20ref%29))
  (if (Components|ComponentHasTag OtherComp "swing_box")
    (Class|BPITrapezeSwing|GrabSwing(Message) OtherActor self)
    (Collision|SetCollisionEnabled (Variables|Default|GetCollider) "NoCollision")))

(event OnComponentEndOverlap(Collider)
  (params (OverlappedComponent :type Primitive%20Component%20Object%20Reference) (OtherActor :type Actor%20Object%20Reference) (OtherComp :type Primitive%20Component%20Object%20Reference) (OtherBodyIndex :type Integer))
  (if (Components|ComponentHasTag OtherComp "swing_box")
    (Utilities|FlowControl|Delay 1.0)
    (Collision|SetCollisionEnabled (Variables|Default|GetCollider) "QueryOnly")))

(event Custom|KeepSwinging
  ;[1 1 1] Setting the cable length, board position, and some initializations
  (CallFunction|MoveForward)
  (Utilities|FlowControl|Delay (Variables|MovingSwing|GetOneWayFullSwingDuration))
  (CallFunction|MoveBackward))

(event EventBeginPlay
  ;[1 1 1] Setting the cable length, board position, and some initializations
  (bind _attachswitch (Variables|Default|GetattachSwitch)
    (:then
      (Transformation|AttachComponentToComponent (Variables|/Game/ThirdPerson/Blueprints/BP_pushCube/BP_switchDoor.BP_switchDoor_C|GetCube _attachswitch) "None" "KeepWorld" "KeepWorld" "KeepWorld" true))
    (:else)))

(fn ConstructionScript)

(fn MoveForward
  (CallFunction|SetBoardYVelocity (Variables|MovingSwing|GetSwingDefaultVelocity)))

(fn MoveBackward
  (CallFunction|SetBoardYVelocity (* (Variables|MovingSwing|GetSwingDefaultVelocity) -1.0)))

(fn SetBoardYVelocity
  (params (New%20Vel%20Y :type Float%20%28double-precision%29))
  (Physics|SetPhysicsLinearVelocity (Variables|Default|GetBoard) (Math|Vector|MakeVector 0.0 (Math|Float|Clamp(Float) New%20Vel%20Y (Variables|Swing|GetBackwardVelocityBoundary) (Variables|Swing|GetForwardVelocityBoundary)) 0.0) true "None"))

(fn AddSwingForce
  (params (SwingTowards :type Vector :default "3.000000,3.000000,3.000000"))
  (Physics|AddForce (Variables|Default|GetBoard) SwingTowards "None" true))