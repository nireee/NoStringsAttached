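; Circus-act seesaw that launches the object on one end when another object lands on the opposite end.
; Left and right box triggers track the occupant of each side that implements BPI_SeeSaw.
; An overlap on either surface reads that side's vertical velocity, taken from the static mesh for cube trigger actors.
; ChoiceForce compares it to FallSpeed and sends the opposite object a high or low push through the interface.
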(event OnComponentBeginOverlap(BoxRight)
  (params (OverlappedComponent :type Primitive%20Component%20Object%20Reference) (OtherActor :type Actor%20Object%20Reference) (OtherComp :type Primitive%20Component%20Object%20Reference) (OtherBodyIndex :type Integer) (bFromSweep :type Boolean) (SweepResult :type Hit%20Result%20Structure%20%28by%20ref%29))
  (if (Utilities|DoesObjectImplementInterface OtherActor "/Game/Blueprints/CircusActs/Interfaces/BPI_SeeSaw.BPI_SeeSaw_C")
    (Variables|Default|SetRightObject OtherActor)))

(event OnComponentEndOverlap(BoxRight)
  (params (OverlappedComponent :type Primitive%20Component%20Object%20Reference) (OtherActor :type Actor%20Object%20Reference) (OtherComp :type Primitive%20Component%20Object%20Reference) (OtherBodyIndex :type Integer))
  (if (Utilities|DoesObjectImplementInterface OtherActor "/Game/Blueprints/CircusActs/Interfaces/BPI_SeeSaw.BPI_SeeSaw_C")
    (Variables|Default|SetRightObject 0)))

(event OnComponentBeginOverlap(BoxLeft)
  (params (OverlappedComponent :type Primitive%20Component%20Object%20Reference) (OtherActor :type Actor%20Object%20Reference) (OtherComp :type Primitive%20Component%20Object%20Reference) (OtherBodyIndex :type Integer) (bFromSweep :type Boolean) (SweepResult :type Hit%20Result%20Structure%20%28by%20ref%29))
  (if (Utilities|DoesObjectImplementInterface OtherActor "/Game/Blueprints/CircusActs/Interfaces/BPI_SeeSaw.BPI_SeeSaw_C")
    (Variables|Default|SetLeftObject OtherActor)))

(event OnComponentEndOverlap(BoxLeft)
  (params (OverlappedComponent :type Primitive%20Component%20Object%20Reference) (OtherActor :type Actor%20Object%20Reference) (OtherComp :type Primitive%20Component%20Object%20Reference) (OtherBodyIndex :type Integer))
  (if (Utilities|DoesObjectImplementInterface OtherActor "/Game/Blueprints/CircusActs/Interfaces/BPI_SeeSaw.BPI_SeeSaw_C")
    (Variables|Default|SetLeftObject 0)))

(event OnComponentBeginOverlap(SurfaceLeft)
  (params (OverlappedComponent :type Primitive%20Component%20Object%20Reference) (OtherActor :type Actor%20Object%20Reference) (OtherComp :type Primitive%20Component%20Object%20Reference) (OtherBodyIndex :type Integer) (bFromSweep :type Boolean) (SweepResult :type Hit%20Result%20Structure%20%28by%20ref%29))
  (bind _rightobject (Variables|Default|GetRightObject))
  (if (and (Utilities|DoesObjectImplementInterface OtherActor "/Game/Blueprints/CircusActs/Interfaces/BPI_SeeSaw.BPI_SeeSaw_C") (Utilities|IsValid (Variables|Default|GetRightObject)))
    (bind _leftobject (Variables|Default|GetLeftObject)
      (:then
        (bind _asbp_cube_trigger_for_see_saw (Utilities|Casting|CastToBP_CubeTriggerForSeeSaw _leftobject)
          (:then
            (Utilities|ChoiceForce _rightobject _rightobject (.z (Transformation|GetComponentVelocity (Variables|/Game/ThirdPerson/Blueprints/EnvironmentObjects/Hidden/BP_ObjectWithWeight.BP_ObjectWithWeight_C|GetStaticMesh _asbp_cube_trigger_for_see_saw)))))
          (:CastFailed
            (Development|PrintString (Utilities|String|ToString(Float) (.z (Transformation|GetVelocity _leftobject))) true true "(R=0.000000,G=0.183330,B=1.000000,A=1.000000)")
            (Utilities|ChoiceForce _rightobject _rightobject (.z (Transformation|GetVelocity _leftobject))))))
      (:else))))

(event OnComponentBeginOverlap(SurfaceRight)
  (params (OverlappedComponent :type Primitive%20Component%20Object%20Reference) (OtherActor :type Actor%20Object%20Reference) (OtherComp :type Primitive%20Component%20Object%20Reference) (OtherBodyIndex :type Integer) (bFromSweep :type Boolean) (SweepResult :type Hit%20Result%20Structure%20%28by%20ref%29))
  (bind _leftobject (Variables|Default|GetLeftObject))
  (if (and (Utilities|DoesObjectImplementInterface OtherActor "/Game/Blueprints/CircusActs/Interfaces/BPI_SeeSaw.BPI_SeeSaw_C") (Utilities|IsValid (Variables|Default|GetLeftObject)))
    (bind _rightobject (Variables|Default|GetRightObject)
      (:then
        (bind _asbp_cube_trigger_for_see_saw (Utilities|Casting|CastToBP_CubeTriggerForSeeSaw _rightobject)
          (:then
            (Development|PrintString (Utilities|String|ToString(Float) (.z (Transformation|GetComponentVelocity (Variables|/Game/ThirdPerson/Blueprints/EnvironmentObjects/Hidden/BP_ObjectWithWeight.BP_ObjectWithWeight_C|GetStaticMesh _asbp_cube_trigger_for_see_saw)))) true true "(R=1.000000,G=0.000000,B=0.018480,A=1.000000)")
            (Utilities|ChoiceForce _leftobject _leftobject (.z (Transformation|GetComponentVelocity (Variables|/Game/ThirdPerson/Blueprints/EnvironmentObjects/Hidden/BP_ObjectWithWeight.BP_ObjectWithWeight_C|GetStaticMesh _asbp_cube_trigger_for_see_saw)))))
          (:CastFailed
            (Utilities|ChoiceForce _leftobject _leftobject (.z (Transformation|GetVelocity _rightobject))))))
      (:else))))

(event EventBeginPlay
  (|CallParentFunction) ; This node is disabled and will not be called.\nDrag off pins to build functionality.
)

(event Collision|EventActorBeginOverlap
  (params (OtherActor :type Actor%20Object%20Reference))
  (|CallParentFunction OtherActor) ; This node is disabled and will not be called.\nDrag off pins to build functionality.
)

(event EventTick
  (params (DeltaSeconds :type Float%20%28single-precision%29))
  (|CallParentFunction DeltaSeconds) ; This node is disabled and will not be called.\nDrag off pins to build functionality.
)

(fn ConstructionScript
  (|CallParentFunction))