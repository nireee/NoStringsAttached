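; ControllerButton is a pressable button that remotely drives BP_Robot, acting as a direction or interact control according to its Direction string.
; Tick maps Direction to a robot yaw and mode, while overlap turns the robot and animates the cube press via a Timeline.
; While overlapped, direction buttons step the robot along its right vector each frame, without delta-time scaling.
; The Interact button instead alternates picking up and leaving pills.
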(event Custom|CheckRobotStatus
  ;[1 1 1] CheckRobotStatus
  (Utilities|FlowControl|Sequence
    (:then_0
      (if (== (Variables|Default|Getdirection) "Up")
        (Variables|Default|SetRobotRot 0.0)
        (Variables|Default|SetMoveIndex (Variables|Default|GetMoveIndex))
        (Variables|Default|Setinteract_button false)
        (Variables|Default|Setonce false)))
    (:then_1
      (if (== (Variables|Default|Getdirection) "Down")
        (Variables|Default|SetRobotRot 1.8e+02)
        (Variables|Default|SetMoveIndex (Variables|Default|GetMoveIndex))
        (Variables|Default|Setinteract_button false)
        (Variables|Default|Setonce false)))
    (:then_2
      (if (== (Variables|Default|Getdirection) "Left")
        (Variables|Default|SetRobotRot -9e+01)
        (Variables|Default|SetMoveIndex (Variables|Default|GetMoveIndex))
        (Variables|Default|Setinteract_button false)
        (Variables|Default|Setonce false)))
    (:then_3
      (if (== (Variables|Default|Getdirection) "Right")
        (Variables|Default|SetRobotRot 9e+01)
        (Variables|Default|SetMoveIndex (Variables|Default|GetMoveIndex))
        (Variables|Default|Setinteract_button false)
        (Variables|Default|Setonce false)))
    (:then_4
      (if (== (Variables|Default|Getdirection) "Interact")
        (Variables|Default|SetRobotRot (.yaw (Transformation|GetActorRotation (Variables|Default|GetRobot))))
        (Variables|Default|SetMoveIndex "0, 0, 0")
        (Variables|Default|Setinteract_button true)))))

(event Custom|UpdateRobotStatus
  (bind _robot (Variables|Default|GetRobot))
  ;[1 1 1] UpdateRobotStatus
  (Transformation|SetActorLocation _robot (+ (Transformation|GetActorLocation _robot) (Variables|Default|GetMoveIndex)) false false))

(event Custom|SetRobotStatus
  (params (rot :type Float%20%28double-precision%29) (obj :type BP%20Robot%20Object%20Reference))
  (bind _returnvalue (Transformation|GetActorRotation obj))
  (Transformation|SetActorRotation obj (Math|Rotator|MakeRotator (.roll _returnvalue) (.pitch _returnvalue) rot))
  (Variables|Default|SetMoveIndex (Transformation|GetActorRightVector obj)))

(event EventBeginPlay
  (bind _returnvalue (Actor|GetActorOfClass "/Game/Blueprints/BP_Robot.BP_Robot_C"))
  (Variables|Default|SetRobot _returnvalue)
  (Variables|Default|Setonce true))

(event Collision|EventActorBeginOverlap
  (params (OtherActor :type Actor%20Object%20Reference))
  (bind _robot (Variables|Default|GetRobot))
  (Variables|Default|Setmoveornot true)
  (CallFunction|SetRobotStatus (Variables|Default|GetRobotRot) (Variables|Default|GetRobot))
  (if (Variables|Default|Getinteract_button)
    (if (Variables|Default|Getonce)
      (Variables|Default|Setpickup (not (Variables|Default|Getpickup)))
      (Variables|Default|Setonce false)
      (if (Variables|Default|Getpickup)
        (Default|PickUpPills _robot)
        (bind _buttonmove_test (Timeline|Timeline Play)
          (:Update
            (Transformation|SetRelativeLocation (Variables|Default|GetCube) (Math|Vector|MakeVector 0.0 0.0 _buttonmove_test) false false)))
        (elif (Variables|Default|Getinteract_button)
          (Default|LeavePills _robot)
          (Timeline|Timeline Play)))
      (else
        (Timeline|Timeline Play)))
    (else
      (Timeline|Timeline Play))))

(event Collision|EventActorEndOverlap
  (params (OtherActor :type Actor%20Object%20Reference))
  (Variables|Default|Setmoveornot false)
  (if (Variables|Default|Getinteract_button)
    (Variables|Default|Setonce true)
    (bind _buttonmove_test (Timeline|Timeline Reverse)
      (:Update
        (Transformation|SetRelativeLocation (Variables|Default|GetCube) (Math|Vector|MakeVector 0.0 0.0 _buttonmove_test) false false)))
    (else
      (Timeline|Timeline Reverse))))

(event EventTick
  (params (DeltaSeconds :type Float%20%28single-precision%29))
  (CallFunction|CheckRobotStatus)
  (if (Variables|Default|Getmoveornot)
    (CallFunction|UpdateRobotStatus)))

(fn ConstructionScript)