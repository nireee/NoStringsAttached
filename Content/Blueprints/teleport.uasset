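; Teleporter actor that moves the player's third person character to a linked destination actor on overlap.
; BeginPlay caches the player character, and ActorBeginOverlap compares the overlapping actor against that cached reference.
; On a match it teleports the player to the Tp2 reference's location without sweeping and prints a debug message.
; The link is one-way, with only location changed and no cooldown.
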(event EventBeginPlay
  (bind _asbp_third_person_character (Utilities|Casting|CastToBP_ThirdPersonCharacter (Game|GetPlayerCharacter 0)))
  (Variables|Default|SetTP_player _asbp_third_person_character))

(event Collision|EventActorBeginOverlap
  (params (OtherActor :type Actor%20Object%20Reference))
  (bind _tp_player (Variables|Default|GetTP_player))
  (if (== OtherActor _tp_player)
    (Transformation|SetActorLocation _tp_player (Transformation|GetActorLocation (Variables|Default|Gettp2)) false true)
    (Development|PrintString "BOUNCE!")))

(event EventTick
  (params (DeltaSeconds :type Float%20%28single-precision%29)))

(fn ConstructionScript)