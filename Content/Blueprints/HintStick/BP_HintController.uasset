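; BP_HintController switches a flashing hint highlight on and off for balance cubes in the level.
; It caches the player character on BeginPlay and uses that character's LevelPostProcessRef to toggle the HintFlash post-process material and its effect flag.
; TiggerHint looks up the cube by index in HintMaps and enables its flash, while cancelHint calls the flash-off directly on its Index argument.
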(event Custom|TiggerHint
  (params (index :type BP%20Can%20See%20Hint%20Trigger%20Object%20Reference))
  (bind _asbp_balance_cube (Utilities|Casting|CastToBP_balance_cube (.Value (Utilities|Map|Find (Variables|Default|GetHintMaps) index))))
  (bind _levelpostprocessref (Variables|/Game/ThirdPerson/Blueprints/BP_ThirdPersonCharacter.BP_ThirdPersonCharacter_C|GetLevelPostProcessRef (Variables|Default|Getplayer))
    (:then
      (Default|ControlPostProcessMaterial _levelpostprocessref true 1) ; Index 0 is PoseFeedback, 1 is HintFlash
      (Variables|/Game/Materials/PostProcess/BP_LevelPostProcess.BP_LevelPostProcess_C|SetHintFlashEffectIsOpen _levelpostprocessref true)
      (Default|SetHintFlashEffect _asbp_balance_cube true))
    (:else)))

(event Custom|cancelHint
  (params (index :type BP%20Balance%20Cube%20Object%20Reference))
  (bind _levelpostprocessref (Variables|/Game/ThirdPerson/Blueprints/BP_ThirdPersonCharacter.BP_ThirdPersonCharacter_C|GetLevelPostProcessRef (Variables|Default|Getplayer))
    (:then
      (Default|ControlPostProcessMaterial _levelpostprocessref false 1) ; Index 0 is PoseFeedback, 1 is HintFlash
      (Variables|/Game/Materials/PostProcess/BP_LevelPostProcess.BP_LevelPostProcess_C|SetHintFlashEffectIsOpen _levelpostprocessref false)
      (Default|SetHintFlashEffect index false))
    (:else)))

(event EventBeginPlay
  (bind _asbp_third_person_character (Utilities|Casting|CastToBP_ThirdPersonCharacter (Game|GetPlayerCharacter 0)))
  (Variables|Default|Setplayer _asbp_third_person_character))

(event Collision|EventActorBeginOverlap
  (params (OtherActor :type Actor%20Object%20Reference)))

(event EventTick
  (params (DeltaSeconds :type Float%20%28single-precision%29)))

(fn ConstructionScript)