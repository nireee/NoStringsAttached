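; BP_Balloon_2 is a balloon VFX actor that rises with physics-driven, randomly varying motion.
; On BeginPlay it gives the Balloon component a random linear damping and picks a random static mesh from StaticMeshList, so instances differ in look and drift speed.
; Each Tick applies a random upward force as an acceleration change, making the lift independent of mass.
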(event EventBeginPlay
  (bind _staticmeshlist (Variables|Default|GetStaticMeshList))
  (Class|PrimitiveComponent|SetLinearDamping (Variables|Default|GetBalloon) (Math|Random|RandomFloat))
  (Components|StaticMesh|SetStaticMesh (Variables|Default|GetBalloon) (Utilities|Array|Get(acopy) _staticmeshlist (Math|Random|RandomIntegerinRange 0 (Utilities|Array|LastIndex _staticmeshlist)))))

(event EventTick
  (params (DeltaSeconds :type Float%20%28single-precision%29))
  (Physics|AddForce (Variables|Default|GetBalloon) (Math|Vector|MakeVector 0.0 0.0 (Math|Random|RandomFloatinRange 1e+02 2e+02)) "None" true))

(fn ConstructionScript)