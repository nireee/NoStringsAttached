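; Level post-process actor that animates a pose-feedback warning (apparently for watched areas) and a hint flash through Material Parameter Collections.
; Tick ramps the warning's time, speed and edge while active, then fades whole strength after it closes, pausing both effects while BeingCaught.
; Hint-flash time advances while open and resets when closed.
; ControlPostProcessMaterial switches indexed post-process materials on or off via blendable weight.
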(event EventBeginPlay
  (Utilities|FlowControl|Sequence
    (:then_0
      (bind _output_get (Variables|Default|SetCurrentWarningTime (Variables|Default|GetTime)))
      (Rendering|Material|SetScalarParameterValue "/Game/Materials/PostProcess/MPC_PoseFeedback.MPC_PoseFeedback" "Time" _output_get :!class /Script/Engine.KismetMaterialLibrary))
    (:then_1
      (bind _output_get_2 (Variables|Default|SetCurrentChangeSpeed (Variables|Default|GetChangeSpeed)))
      (Rendering|Material|SetScalarParameterValue "/Game/Materials/PostProcess/MPC_PoseFeedback.MPC_PoseFeedback" "ChangeSpeed" _output_get_2 :!class /Script/Engine.KismetMaterialLibrary))
    (:then_2
      (bind _output_get_3 (Variables|Default|SetCurrentChangeOutsideEdge (Variables|Default|GetChangeOutsideEdge)))
      (Rendering|Material|SetScalarParameterValue "/Game/Materials/PostProcess/MPC_PoseFeedback.MPC_PoseFeedback" "ChangeOutsideEdge" _output_get_3 :!class /Script/Engine.KismetMaterialLibrary))
    (:then_3
      (bind _output_get_4 (Variables|Default|SetCurrentWarningWholeStrength (Variables|Default|GetWarningWholeStrength)))
      (Rendering|Material|SetScalarParameterValue "/Game/Materials/PostProcess/MPC_PoseFeedback.MPC_PoseFeedback" "WholeStrength" _output_get_4 :!class /Script/Engine.KismetMaterialLibrary))
    (:then_4
      (Variables|Default|SetEnteredWatchingAreaOnce false))
    (:then_5
      (Variables|Default|SetBeingCaught false))))

(event EventTick
  (params (DeltaSeconds :type Float%20%28single-precision%29))
  (bind _returnvalue (Utilities|Time|GetWorldDeltaSeconds))
  (bind _returnvalue_2 (Utilities|Time|GetWorldDeltaSeconds))
  (if (not (Variables|Default|GetBeingCaught))
    (Utilities|FlowControl|Sequence
      (:then_0
        (if (Variables|Default|GetPoseFeedbackEffectIsOpen)
          (Utilities|FlowControl|Sequence
            (:then_0
              (Variables|Default|SetEnteredWatchingAreaOnce true))
            (:then_1
              (bind _output_get (Variables|Default|SetCurrentWarningTime (+ _returnvalue (Variables|Default|GetCurrentWarningTime))))
              (Rendering|Material|SetScalarParameterValue "/Game/Materials/PostProcess/MPC_PoseFeedback.MPC_PoseFeedback" "Time" _output_get :!class /Script/Engine.KismetMaterialLibrary))
            (:then_2
              (Variables|Default|SetCurrentChangeSpeed (+ (* _returnvalue (Variables|Default|GetSpeedOfChangeSpeed)) (Variables|Default|GetCurrentChangeSpeed)))
              (Rendering|Material|SetScalarParameterValue "/Game/Materials/PostProcess/MPC_PoseFeedback.MPC_PoseFeedback" "ChangeSpeed" (Variables|Default|GetCurrentChangeSpeed) :!class /Script/Engine.KismetMaterialLibrary))
            (:then_3
              (bind _output_get_2 (Variables|Default|SetCurrentChangeOutsideEdge (+ (* _returnvalue (Variables|Default|GetSpeedOfChangeOutsideEdge)) (Variables|Default|GetCurrentChangeOutsideEdge))))
              (Rendering|Material|SetScalarParameterValue "/Game/Materials/PostProcess/MPC_PoseFeedback.MPC_PoseFeedback" "ChangeOutsideEdge" _output_get_2 :!class /Script/Engine.KismetMaterialLibrary)))
          (else
            (Utilities|FlowControl|Sequence
              (:then_0
                (Utilities|FlowControl|DoOnce false
                  (:Completed
                    (bind _output_get_3 (Variables|Default|SetCurrentWarningTime (Variables|Default|GetTime)))
                    (Rendering|Material|SetScalarParameterValue "/Game/Materials/PostProcess/MPC_PoseFeedback.MPC_PoseFeedback" "Time" _output_get_3 :!class /Script/Engine.KismetMaterialLibrary))))
              (:then_1
                (Utilities|FlowControl|DoOnce false
                  (:Completed
                    (bind _output_get_4 (Variables|Default|SetCurrentChangeSpeed (Variables|Default|GetChangeSpeed)))
                    (Rendering|Material|SetScalarParameterValue "/Game/Materials/PostProcess/MPC_PoseFeedback.MPC_PoseFeedback" "ChangeSpeed" _output_get_4 :!class /Script/Engine.KismetMaterialLibrary))))
              (:then_2
                (Utilities|FlowControl|DoOnce false
                  (:Completed
                    (bind _output_get_5 (Variables|Default|SetCurrentChangeOutsideEdge (Variables|Default|GetChangeOutsideEdge)))
                    (Rendering|Material|SetScalarParameterValue "/Game/Materials/PostProcess/MPC_PoseFeedback.MPC_PoseFeedback" "ChangeOutsideEdge" _output_get_5 :!class /Script/Engine.KismetMaterialLibrary))))
              (:then_3
                (if (Variables|Default|GetEnteredWatchingAreaOnce)
                  (if (> (Variables|Default|GetCurrentWarningWholeStrength) 0.0)
                    (bind _output_get_6 (Variables|Default|SetCurrentWarningWholeStrength (- (Variables|Default|GetCurrentWarningWholeStrength) (* (/ (Variables|Default|GetWarningWholeStrength) (Variables|Default|GetWarningWholeStrengthFadingTime)) _returnvalue_2))))
                    (Rendering|Material|SetScalarParameterValue "/Game/Materials/PostProcess/MPC_PoseFeedback.MPC_PoseFeedback" "WholeStrength" _output_get_6 :!class /Script/Engine.KismetMaterialLibrary)
                    (Development|PrintString (Utilities|String|ToString(Float) _output_get_6) true true "(R=0.000000,G=0.660000,B=1.000000,A=1.000000)" _output_get_6)
                    (else
                      (Variables|Default|SetEnteredWatchingAreaOnce false)
                      (bind _output_get_7 (Variables|Default|SetCurrentWarningWholeStrength (Variables|Default|GetWarningWholeStrength)))
                      (Rendering|Material|SetScalarParameterValue "/Game/Materials/PostProcess/MPC_PoseFeedback.MPC_PoseFeedback" "WholeStrength" _output_get_7 :!class /Script/Engine.KismetMaterialLibrary)
                      (Development|PrintString (Utilities|String|ToString(Float) _output_get_7))))))))))
      (:then_1
        (if (Variables|Default|GetHintFlashEffectIsOpen)
          (bind _output_get_8 (Variables|Default|SetCurrentSeeingHintTime (+ _returnvalue_2 (Variables|Default|GetCurrentSeeingHintTime))))
          (Rendering|Material|SetScalarParameterValue "/Game/Materials/PostProcess/MPC_HintFlash.MPC_HintFlash" "Time" _output_get_8 :!class /Script/Engine.KismetMaterialLibrary)
          (else
            (bind _output_get_9 (Variables|Default|SetCurrentSeeingHintTime (Variables|Default|GetTime)))
            (Rendering|Material|SetScalarParameterValue "/Game/Materials/PostProcess/MPC_HintFlash.MPC_HintFlash" "Time" _output_get_9 :!class /Script/Engine.KismetMaterialLibrary)))))))

(event Collision|EventActorBeginOverlap
  (params (OtherActor :type Actor%20Object%20Reference)))

(fn ConstructionScript)

(fn ControlPostProcessMaterial
  (params (PostProcessMaterialIsOpen :type Boolean) (IndexOfPostProcessMaterials :type Integer))
  (bind _pp (Variables|Default|GetPP))
  (bind _settings (Variables|/Script/Engine.PostProcessComponent|GetSettings _pp))
  (bind _weightedblendables (Utilities|Struct|BreakPostProcessSettings _settings))
  (bind _array (Utilities|Struct|BreakWeightedBlendables _weightedblendables))
  (bind _output (Utilities|Array|Get(acopy) _array IndexOfPostProcessMaterials))
  (Utilities|Struct|SetmembersinWeightedBlendable _output (Math|Conversions|ToFloat(Boolean) PostProcessMaterialIsOpen) (.Object (Utilities|Struct|BreakWeightedBlendable _output)))
  (Utilities|Struct|SetmembersinWeightedBlendables _weightedblendables _array))